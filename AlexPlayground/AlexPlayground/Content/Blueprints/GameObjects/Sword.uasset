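; Sword is a grabbable game object Blueprint that extends a parent's grab and release behavior.
; On grab and on release it calls the parent event, then turns physics simulation on its Blade component off while held and back on when released.
; It supplies fixed attach position and rotation offsets, shifting the sword along Z and tilting it when attached.
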(event EventOnGrab
  (|CallParentFunction)
  (Physics|SetSimulatePhysics (Variables|Default|GetBlade) false))

(event EventOnRelease
  (|CallParentFunction)
  (Physics|SetSimulatePhysics (Variables|Default|GetBlade) true))

(fn ConstructionScript)

(fn GetAttachPositionOffset
  (return "0, 0,-100.000000"))

(fn GetAttachRotationOffset
  (return "0,-45.000000, 0"))