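; Shuriken is a grabbable throwing-weapon object that sticks to the actor it hits.
; Grab and release extend the parent's handlers, switching mesh physics off and on, and fixed offsets define its attach pose.
; A mesh hit stops physics and attaches it to that actor, snapping to its location and rotation rather than the impact point.
; The sword ribbon particle starts deactivated; release calls emitter enable with name None.
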(event OnComponentHit(Mesh)
  (params (HitComponent :type Primitive%20Component%20Object%20Reference) (OtherActor :type Actor%20Object%20Reference) (OtherComp :type Primitive%20Component%20Object%20Reference) (NormalImpulse :type Vector :default "0, 0, 0") (Hit :type Hit%20Result%20Structure%20%28by%20ref%29))
  (Physics|SetSimulatePhysics (Variables|Default|GetMesh) false)
  (Transformation|AttachActorToActor OtherActor "None" "SnapToTarget" "SnapToTarget" "KeepRelative" true))

(event EventOnGrab
  (|CallParentFunction)
  (Physics|SetSimulatePhysics (Variables|Default|GetMesh) false))

(event EventOnRelease
  (|CallParentFunction)
  (Physics|SetSimulatePhysics (Variables|Default|GetMesh) true)
  (Effects|Components|ParticleSystem|SetEmitterEnable (Variables|Default|GetP_Sword_Ribbon) "None" true))

(event EventBeginPlay
  (Components|Activation|Deactivate (Variables|Default|GetP_Sword_Ribbon)))

(fn ConstructionScript)

(fn GetAttachPositionOffset
  (return "50.000000,-35.000000,0.000000"))

(fn GetAttachRotationOffset
  (return "0.000000,0.000000, 0"))