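; VR player pawn with an eye-level tracking origin, stick locomotion, cooldown-gated turning and a left-trigger headset reset.
; Tick moves the pawn with sweep relative to camera yaw and turns it in steps when the stick nears full deflection.
; Grips run short hand traces to attach GrabbableObjectBase actors using their own offsets, detaching them on release.
; RotateTorso is empty, and RotateToMatchView is never called here.
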(event EventBeginPlay
  (Class|HeadMountedDisplayFunctionLibrary|SetTrackingOrigin "Eye"))

(event EventTick
  (params (DeltaSeconds :type Float%20%28single-precision%29))
  (CallFunction|MovePlayer DeltaSeconds)
  (bind _rotatedthisframe (CallFunction|RotatePlayer DeltaSeconds))
  (if _rotatedthisframe
    (Utilities|FlowControl|Delay (Variables|Default|GetRotationCooldown))
    (Variables|Default|SetCanRotateThisFrame true))
  (CallFunction|RotateTorso))

(event Input|KeyboardEvents|MotionControllerLeftTrigger
  (params (Key :type Key%20Structure :default "None"))
  (:Pressed
    (Class|HeadMountedDisplayFunctionLibrary|ResetOrientationandPosition 0.0 "OrientationAndPosition")))

(event Input|KeyboardEvents|MotionControllerRightTrigger
  (params (Key :type Key%20Structure :default "None")))

(event Input|KeyboardEvents|MotionControllerLeftGrip1
  (params (Key :type Key%20Structure :default "None"))
  (bind _lefthand (Variables|Default|GetLeftHand))
  (:Pressed
    (CallFunction|GrabObject _lefthand))
  (:Released
    (CallFunction|ReleaseObject _lefthand)))

(event Input|KeyboardEvents|MotionControllerRightGrip1
  (params (Key :type Key%20Structure :default "None"))
  (bind _righthand (Variables|Default|GetRightHand))
  (:Pressed
    (CallFunction|GrabObject _righthand))
  (:Released
    (CallFunction|ReleaseObject _righthand)))

(fn ConstructionScript)

(fn GrabObject
  (params (GrabbingHand :type Scene%20Component%20Object%20Reference))
  (bind _returnvalue (Transformation|GetWorldLocation GrabbingHand))
  (bind (_outhit _returnvalue_2) (Collision|LineTraceByChannel _returnvalue (+ _returnvalue (* (Math|Vector|GetForwardVector GrabbingHand) 1e+01)) "TraceTypeQuery3" false 0 "None"))
  (if _returnvalue_2
    (bind _asgrabbable_object_base (Utilities|Casting|CastToGrabbableObjectBase (.HitActor (Collision|BreakHitResult _outhit))))
    (Default|OnGrab _asgrabbable_object_base)
    (Transformation|AttachComponentToComponent (.HitActor (Collision|BreakHitResult _outhit)) GrabbingHand "None" "SnapToTarget" "SnapToTarget" "KeepWorld" true)
    (bind _rotationoffset (Default|GetAttachRotationOffset _asgrabbable_object_base))
    (Transformation|AddActorLocalRotation (.HitActor (Collision|BreakHitResult _outhit)) (Math|Rotator|MakeRotator (.x _rotationoffset) (.y _rotationoffset) (.z _rotationoffset)) false false)
    (bind _positionoffset (Default|GetAttachPositionOffset _asgrabbable_object_base))
    (Transformation|AddActorLocalOffset (.HitActor (Collision|BreakHitResult _outhit)) _positionoffset false true)))

(fn ReleaseObject
  (params (ReleasingHand :type Scene%20Component%20Object%20Reference))
  (bind _returnvalue (Components|GetChildComponent ReleasingHand 0))
  (Utilities|IsValid _returnvalue
    (:Is%20Valid
      (bind _asgrabbable_object_base (Utilities|Casting|CastToGrabbableObjectBase (Components|GetOwner _returnvalue)))
      (Default|OnRelease _asgrabbable_object_base)
      (Transformation|DetachFromComponent _returnvalue "KeepWorld" "KeepWorld" "KeepWorld" true))))

(fn MovePlayer
  (params (DeltaTime :type Float%20%28single-precision%29))
  (Transformation|SetActorLocation (+ (Transformation|GetActorLocation) (Math|Vector|RotateVectorAroundAxis (* (* (Math|Vector|MakeVector (* (Class|Actor|GetInputAxisKeyValue) -1.0) (Class|Actor|GetInputAxisKeyValue) 0.0) (Variables|Default|GetMovementSpeed)) DeltaTime) (.yaw (Transformation|GetWorldRotation (Variables|Default|GetVRCamera))) "0, 0,1.000000")) true false))

(fn RotatePlayer
  (params (DeltaTime :type Float%20%28single-precision%29))
  (if (Variables|Default|GetCanRotateThisFrame)
    (if (or (Math|Float|NearlyEqual(Float) (Class|Actor|GetInputAxisKeyValue) 1.0 0.2) (Math|Float|NearlyEqual(Float) (Class|Actor|GetInputAxisKeyValue) -1.0 0.2))
      (Class|Actor|AddActorWorldRotation (Math|Rotator|MakeRotator 0.0 0.0 (* (Class|Actor|GetInputAxisKeyValue) (Variables|Default|GetRotationSpeed) DeltaTime)))
      (Variables|Default|SetCanRotateThisFrame false)
      (return true))))

(fn RotatetoMatchView
  (if (Game|Player|IsInputKeyDown (Game|GetPlayerController 0) "MotionController_Left_FaceButton1")
    (Class|Actor|AddActorWorldRotation (Math|Rotator|MakeRotator 0.0 0.0 (* (- (.yaw (Transformation|GetWorldRotation (Variables|Default|GetVRCamera))) (Variables|Default|GetLastZRotation)) -1.0))))
  (Variables|Default|SetLastZRotation (.yaw (Transformation|GetWorldRotation (Variables|Default|GetVRCamera)))))

(fn RotateTorso)